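; Enemy spawner actor that keeps spawning random enemies for as long as it runs.
; BeginPlay starts an endless loop that waits SpawnDelay, then calls SpawnEnemy.
; SpawnEnemy picks a random class from EnemyClasses and spawns it with SpawnerMechanism's rotation and scale.
; RandomizeSpawn offsets it from the mechanism by SpawnLocation's X and Y, with Z randomized within plus or minus SpawnRange.
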(event `self.ReceiveBeginPlay`
  (`KismetSystemLibrary.RetriggerableDelay` (`self.SpawnDelay`) :!label _label)
  (`self.SpawnEnemy`)
  (goto _label))

(event `self.ReceiveTick`
  (params (DeltaSeconds :type "Float (single-precision)")))

(event `SpawnEnemy`
  ;[1 1 1] Spawn new enemy
  (bind _newlocation (`self.RandomizeSpawn` (`self.SpawnLocation`) (`self.SpawnRange`)))
  (`|SpawnActorFromClass` (`KismetArrayLibrary.Array_Random` (`self.EnemyClasses`)) (`KismetMathLibrary.MakeTransform` (+ _newlocation (.location (`SceneComponent.K2_GetComponentToWorld` (`self.SpawnerMechanism`)))) (.rotation (`SceneComponent.K2_GetComponentToWorld` (`self.SpawnerMechanism`))) (.scale (`SceneComponent.K2_GetComponentToWorld` (`self.SpawnerMechanism`)))) "Undefined" "OverrideRootScale" null null))

(fn `RandomizeSpawn`
  (params (SpawnLocation :type "Vector Structure") (SpawnRange :type "Float (double-precision)"))
  (returns (NewLocation :type "Vector Structure"))
  (return (`KismetMathLibrary.MakeVector` (.x SpawnLocation) (.y SpawnLocation) (`KismetMathLibrary.RandomFloatInRange` (* -1 SpawnRange) SpawnRange))))

(fn `UserConstructionScript`)