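; BP_PlayerShadow is an actor that mirrors the player pawn's height from a fixed horizontal offset.
; On BeginPlay it moves to the player's location shifted along X by XOffset, intended as the opposite side of the player.
; Each Tick it keeps its own X and Y while copying the player's Z, and destroys itself once BP_GameMode reports GameOver.
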(event `self.ReceiveBeginPlay`
  (bind (_returnvalue_x _returnvalue_y _returnvalue_z) (`KismetMathLibrary.BreakVector` (`self.K2_GetActorLocation` (`GameplayStatics.GetPlayerPawn` 0))))
  ;[1 1 1] Start on the exact opposite side of the player
  (`self.K2_SetActorLocation` (`KismetMathLibrary.MakeVector` (+ (`self.XOffSet`) _returnvalue_x) _returnvalue_y _returnvalue_z)))

(event `self.ReceiveTick`
  (params (DeltaSeconds :type "Float (single-precision)"))
  (bind (_returnvalue_x _returnvalue_y) (`KismetMathLibrary.BreakVector` (`self.K2_GetActorLocation`)))
  (bind (_returnvalue_x_2 _returnvalue_y_2 _returnvalue_z) (`KismetMathLibrary.BreakVector` (`self.K2_GetActorLocation` (`GameplayStatics.GetPlayerPawn` 0))))
  ;[1 1 1] Follow the player as they move
  (bind _asbp_game_mode (cast `/Game/Blueprints/BP_GameMode` (`GameplayStatics.GetGameMode`)))
  (if (`/Game/Blueprints/BP_GameMode.GameOver` _asbp_game_mode)
    (`self.K2_DestroyActor`)
    (else
      (`self.K2_SetActorLocation` (`KismetMathLibrary.MakeVector` _returnvalue_x _returnvalue_y _returnvalue_z)))))

(fn `UserConstructionScript`)