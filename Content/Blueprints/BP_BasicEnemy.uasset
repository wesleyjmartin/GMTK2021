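; Basic enemy actor that moves at a constant velocity and can damage the player or be shot for points.
; Each tick it moves itself with a swept location update and destroys itself if BP_GameMode flags game over.
; Collider overlap with the player destroys the enemy and applies damage.
; Overlap with a player bullet destroys both, adding points to the game mode's score and refreshing the player's HUD.
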(event `self.ReceiveActorBeginOverlap`
  (params (OtherActor :type "Actor Object Reference")))

(event `self.ReceiveTick`
  (params (DeltaSeconds :type "Float (single-precision)"))
  (`self.MoveEnemy` DeltaSeconds)
  (bind _asbp_game_mode (cast `/Game/Blueprints/BP_GameMode` (`GameplayStatics.GetGameMode`)))
  (if (`/Game/Blueprints/BP_GameMode.GameOver` _asbp_game_mode)
    (`self.K2_DestroyActor`)))

(event `self.Collider.OnComponentBeginOverlap`
  (params (OverlappedComponent :type "PrimitiveComponent Object Reference") (OtherActor :type "Actor Object Reference") (OtherComp :type "PrimitiveComponent Object Reference") (OtherBodyIndex :type Integer) (bFromSweep :type Boolean) (SweepResult :type "HitResult Structure (by ref)"))
  (cast `/Game/Blueprints/BP_Player` OtherActor
    (:`then`
      (`self.K2_DestroyActor`)
      (bind _asbp_player (cast `/Game/Blueprints/BP_Player` (`GameplayStatics.GetPlayerPawn` 0)))
      (`GameplayStatics.ApplyDamage` _asbp_player 1.0))
    (:`CastFailed`
      (bind _asbp_player_bullet (cast `/Game/Blueprints/BP_PlayerBullet` OtherActor))
      (`self.K2_DestroyActor` _asbp_player_bullet)
      (`self.K2_DestroyActor`)
      (`self.AddPoints` (`self.PointVal`)))))

(fn `AddPoints`
  (params (PointVal :type Integer))
  (bind _asbp_game_mode (cast `/Game/Blueprints/BP_GameMode` (`GameplayStatics.GetGameMode`)))
  (bind _output_get (set `/Game/Blueprints/BP_GameMode.Score` (+ (`/Game/Blueprints/BP_GameMode.Score` _asbp_game_mode) PointVal) _asbp_game_mode))
  (bind _asbp_player (cast `/Game/Blueprints/BP_Player` (`GameplayStatics.GetPlayerPawn` 0)))
  (`/Game/Blueprints/BP_UI_HUD.UpdateScore` (`/Game/Blueprints/BP_Player.HUD REF` _asbp_player) _output_get))

(fn `MoveEnemy`
  (params (`Delta Time` :type "Float (double-precision)"))
  (`self.K2_SetActorLocation` (+ (`self.K2_GetActorLocation`) (* (`self.Velocity`) `Delta Time`)) true))

(fn `UserConstructionScript`)