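; BP_GameMode is a game mode that handles level start and player death.
; On BeginPlay it fades the camera in from black and plays a flying sound cue.
; Its PlayerKilled event prints a death message, fades out while holding, plays a fail sound, then reopens the current level by name after a short delay to restart it.
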(event `self.ReceiveBeginPlay`
  ;[1 1 1] Fade in camera when game starts
  (`PlayerCameraManager.StartCameraFade` :`self` (`GameplayStatics.GetPlayerCameraManager` 0) :`FromAlpha` 1.0 :`Duration` 1.5)
  (`GameplayStatics.PlaySound2D` "/Game/Assets/Wes/Flying1_Cue.Flying1_Cue" 1.0 1.0 0.0 null null))

(event `PlayerKilled`
  ;[1 1 1] Player has been killed. Fade out and restart the level
  (`KismetSystemLibrary.PrintString` "Ur dead lol")
  (`PlayerCameraManager.StartCameraFade` :`self` (`GameplayStatics.GetPlayerCameraManager` 0) :`ToAlpha` 1.0 :`Duration` 1.0 :`bHoldWhenFinished` true)
  (`GameplayStatics.PlaySound2D` "/Game/Assets/Wes/Fail1_Cue.Fail1_Cue" 1.0 1.0 0.0 null null)
  (`KismetSystemLibrary.Delay` 3.0)
  (bind _returnvalue (`GameplayStatics.GetCurrentLevelName` true))
  (`GameplayStatics.OpenLevel` (`KismetStringLibrary.Conv_StringToName` _returnvalue)))

(fn `UserConstructionScript`)