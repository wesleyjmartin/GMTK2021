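; BP_HomingEnemy is an enemy ship that homes in on the player and has a point value of 100, set on BeginPlay.
; MoveEnemy turns the EnemyShip component to face BP_Player, with a -90 pitch offset, and moves the actor straight toward it with a swept, delta-time-scaled step.
; Its own Tick is disabled, so nothing in this graph calls MoveEnemy.
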(event `self.ReceiveBeginPlay`
  (`parent.ReceiveBeginPlay`)
  (set `self.PointVal` 100))

(fn `MoveEnemy`
  (params (`Delta Time` :type "Float (double-precision)"))
  (locals (Player :type "Object Object Reference" :default "Blueprint'/Game/Blueprints/BP_Player.BP_Player'"))
  (bind _returnvalue (`self.K2_GetActorLocation`))
  (bind _asbp_player (cast `/Game/Blueprints/BP_Player` (`GameplayStatics.GetPlayerPawn` 0)))
  (bind _returnvalue_2 (`KismetMathLibrary.FindLookAtRotation` _returnvalue (`self.K2_GetActorLocation` _asbp_player)))
  (`SceneComponent.K2_SetWorldRotation` (`self.Enemy_Ship`) (`KismetMathLibrary.MakeRotator` (.roll _returnvalue_2) (+ (.pitch _returnvalue_2) -90.0) (.yaw _returnvalue_2)) false false)
  (`self.K2_SetActorLocation` (+ (* (`KismetMathLibrary.GetForwardVector` _returnvalue_2) (* `Delta Time` (`self.spped`))) _returnvalue) true))

(fn `UserConstructionScript`
  (`parent.UserConstructionScript`))